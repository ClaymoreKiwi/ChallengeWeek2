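; Trigger volume Blueprint that blends the player's view to another camera and plays crowd chatter while overlapped.
; On begin overlap, a ThirdPersonCharacter's PlayerController blends to the first actor of the Cam class; on end overlap it blends back to the character using the same BlendTime.
; The 2D sound starts and stops on separate sequence branches without the character check, so any overlapping actor triggers it.
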(event `self.OverlapVolume.OnComponentBeginOverlap`
  (params (OverlappedComponent :type "PrimitiveComponent Object Reference") (OtherActor :type "Actor Object Reference") (OtherComp :type "PrimitiveComponent Object Reference") (OtherBodyIndex :type Integer) (bFromSweep :type Boolean) (SweepResult :type "HitResult Structure (by ref)"))
  (`|ExecutionSequence`
    (:`then_0`
      (bind _asthird_person_character (cast `/Game/ThirdPersonBP/Blueprints/ThirdPersonCharacter` OtherActor))
      (if (`KismetSystemLibrary.IsValid` _asthird_person_character)
        (bind _asplayer_controller (cast `PlayerController` (`Pawn.GetController` _asthird_person_character)))
        (if (`KismetSystemLibrary.IsValid` _asplayer_controller)
          (bind _returnvalue (`GameplayStatics.GetActorOfClass` "/Game/Bryce_Folder/Cam.Cam_C"))
          (`PlayerController.SetViewTargetWithBlend` _asplayer_controller _returnvalue (`self.blendTime`) "VTBlend_Linear" 0.0 false))))
    (:`then_1`
      (bind _returnvalue_2 (`GameplayStatics.SpawnSound2D` "/Game/Bryce_Folder/crowd_talking-6762.crowd_talking-6762" 1.0 1.0 0.0 null))
      (set `self.sound` _returnvalue_2))))

(event `self.OverlapVolume.OnComponentEndOverlap`
  (params (OverlappedComponent :type "PrimitiveComponent Object Reference") (OtherActor :type "Actor Object Reference") (OtherComp :type "PrimitiveComponent Object Reference") (OtherBodyIndex :type Integer))
  (`|ExecutionSequence`
    (:`then_0`
      (bind _asthird_person_character (cast `/Game/ThirdPersonBP/Blueprints/ThirdPersonCharacter` OtherActor))
      (if (`KismetSystemLibrary.IsValid` _asthird_person_character)
        (bind _asplayer_controller (cast `PlayerController` (`Pawn.GetController` _asthird_person_character)))
        (if (`KismetSystemLibrary.IsValid` _asplayer_controller)
          (`PlayerController.SetViewTargetWithBlend` _asplayer_controller _asthird_person_character (`self.blendTime`) "VTBlend_Linear" 0.0 false))))
    (:`then_1`
      (`AudioComponent.Stop` (`self.sound`)))))

(fn `UserConstructionScript`)