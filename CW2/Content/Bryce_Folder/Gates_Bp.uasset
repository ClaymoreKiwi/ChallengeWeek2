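; Gate actor that lowers when interacted with and shows an on-screen prompt to a nearby ThirdPersonCharacter.
; Its Interact function fires an event that plays the Movement timeline, subtracting the track value from the current location each update, so movement accumulates per frame.
; Box overlaps create and remove the Interact_Bp widget.
; The Interact input briefly sets the widget's pressed state, separately from the movement.
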(event `interacingEvent`
  ;[1 1 1] Moves the gate down
  (bind (_direction _newtrack_0) (`Timeline|Movement` :!via `PlayFromStart`)
    (:`Update`
      (`self.K2_SetActorLocation` (- (`self.K2_GetActorLocation`) _newtrack_0)))))

(event `self.ReceiveBeginPlay`)

(event `InputAction|Interact`
  (params (Key :type "Key Structure"))
  (:`Pressed`
    (set `/Game/Bryce_Folder/Interact_Bp.IsPressed` true (stale `self.Box.OnComponentBeginOverlap` _returnvalue))
    (`KismetSystemLibrary.Delay` 0.2)
    (set `/Game/Bryce_Folder/Interact_Bp.IsPressed` false (stale `self.Box.OnComponentBeginOverlap` _returnvalue))))

(event `self.Box.OnComponentBeginOverlap`
  (params (OverlappedComponent :type "PrimitiveComponent Object Reference") (OtherActor :type "Actor Object Reference") (OtherComp :type "PrimitiveComponent Object Reference") (OtherBodyIndex :type Integer) (bFromSweep :type Boolean) (SweepResult :type "HitResult Structure (by ref)"))
  (cast `/Game/ThirdPersonBP/Blueprints/ThirdPersonCharacter` OtherActor)
  ;[1 1 1] Add and remove prompt
  (bind _returnvalue (`|CreateWidget` "/Game/Bryce_Folder/Interact_Bp.Interact_Bp_C"))
  (`UserWidget.AddToViewport` _returnvalue 0))

(event `self.Box.OnComponentEndOverlap`
  (params (OverlappedComponent :type "PrimitiveComponent Object Reference") (OtherActor :type "Actor Object Reference") (OtherComp :type "PrimitiveComponent Object Reference") (OtherBodyIndex :type Integer))
  (cast `/Game/ThirdPersonBP/Blueprints/ThirdPersonCharacter` OtherActor)
  ;[1 1 1] Add and remove prompt
  (`Widget.RemoveFromParent` (stale `self.Box.OnComponentBeginOverlap` _returnvalue)))

(fn `Interact`
  (params (Interactor :type "Character Object Reference"))
  (returns (success :type Boolean))
  (`self.interacingEvent`)
  (return false))

(fn `UserConstructionScript`)